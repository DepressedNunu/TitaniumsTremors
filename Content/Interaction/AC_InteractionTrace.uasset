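; Interaction component that detects whether the mouse cursor points at a BP_InteractionArea actor.
; Every tick it deprojects player 0's cursor and runs a debug-drawn Visibility line trace out to Length.
; A new hit actor updates FocusActor and passes an exact-class match to TraceInteractionArea, which has an empty body here.
; A miss passes false every tick without clearing FocusActor, so re-hovering the same actor sends no new result.
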(event EventTick
  (params (DeltaSeconds :type Float%20%28single-precision%29))
  (CallFunction|Trace))

(fn Trace
  (bind _returnvalue (Game|GetPlayerController 0))
  (bind (_worldlocation _worlddirection _returnvalue_2) (Game|Player|ConvertMouseLocationToWorldSpace _returnvalue))
  (bind (_outhit _returnvalue_3) (Collision|LineTraceByChannel _worldlocation (+ _worldlocation (* _worlddirection (Variables|Default|GetLength))) "TraceTypeQuery1" false 0 "ForDuration"))
  (if _returnvalue_3
    (if (!= (Variables|Default|GetFocusActor) (.HitActor (Collision|BreakHitResult _outhit)))
      (Variables|Default|SetFocusActor (.HitActor (Collision|BreakHitResult _outhit)))
      (CallFunction|TraceInteractionArea (== (Utilities|GetClass (.HitActor (Collision|BreakHitResult _outhit))) "/Game/Interaction/InteractionArea/BP_InteractionArea.BP_InteractionArea_C")))
    (else
      (CallFunction|TraceInteractionArea false))))

(fn TraceInteractionArea
  (params (Trace :type Boolean)))